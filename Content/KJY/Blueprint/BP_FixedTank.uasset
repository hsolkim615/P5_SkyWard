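; BP_FixedTank is a stationary tank enemy Blueprint whose combat logic is unfinished: its BeginPlay, overlap, Spawn and pawn-sensing events are all empty.
; Disconnected fragments sketch helicopter detection, look-at aiming, a gun line trace from the BulletLoc socket and timed projectile spawning, but none of them run.
; The only complete logic is GetLocation, which computes a ballistic position from initial velocity and time under fixed gravity, offset from the mesh location.
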(event `Spawn`)

(event `self.ReceiveBeginPlay`)

(event `self.pawnSensing.OnSeePawn`
  (params (Pawn :type "Pawn Object Reference")))

(fn `GetLocation`
  (params (u :type "Vector Structure") (t :type "Float (double-precision)"))
  (returns (location :type "Vector Structure"))
  (bind _returnvalue_location (`KismetMathLibrary.BreakTransform` (`SceneComponent.K2_GetComponentToWorld` (`self.Mesh`))))
  (return (+ (* u t) (`KismetMathLibrary.MakeVector` 0.0 0.0 (* 0.5 -980.0 t t)) _returnvalue_location)))

(fn `UserConstructionScript`)